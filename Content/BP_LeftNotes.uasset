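; BP_LeftNotes is a note actor that travels along the LeftLane spline of a referenced Erhu actor.
; MoveNote plays a timeline with its rate scaled by the inverse of TimeToComplete.
; Each update maps the timeline track to a distance along the spline, then applies that point's world location and rotation, using the Sphere's relative scale as the actor scale.
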(event `self.MoveNote`
  (bind _leftlane (`/Game/BP_ErhuActor.LeftLane` (`self.ErhuActor`)))
  (`TimelineComponent.SetPlayRate` (`self.Timeline`) (/ 1.0 (`self.TimeToComplete`)))
  (bind (_direction _newtrack_0) (`Timeline|Timeline`)
    (:`Update`
      (bind _returnvalue (`KismetMathLibrary.Lerp` 0.0 (`SplineComponent.GetSplineLength` (`/Game/BP_ErhuActor.LeftLane` (`self.ErhuActor`))) _newtrack_0))
      (`self.K2_SetActorTransform` (`KismetMathLibrary.MakeTransform` (`SplineComponent.GetLocationAtDistanceAlongSpline` _leftlane _returnvalue "World") (`SplineComponent.GetRotationAtDistanceAlongSpline` _leftlane _returnvalue "World") (`SceneComponent.RelativeScale3D` (`self.Sphere`)))))))

(fn `UserConstructionScript`
  (`parent.UserConstructionScript`))