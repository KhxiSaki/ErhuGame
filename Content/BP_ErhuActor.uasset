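; Erhu rhythm minigame pawn with a left and right note lane, which returns control to the third-person character and destroys itself when the song ends.
; After a countdown, it plays the song and watches MetaSound cue-point labels to spawn moving notes per lane.
; Bullseye overlaps flag hittable notes, so pressing F flashes the bullseye and scores, while destroyer volumes remove passing notes.
; Difficulty currently only affects debug prints.
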(event `self.ReceiveTick`
  (params (DeltaSeconds :type "Float (single-precision)"))
  ; Tick: Checking score
  (`KismetSystemLibrary.PrintString` (`|GetEnumeratorNameAsString` (`self.DifficultyToPlay`))))

(event `self.ReceiveBeginPlay`
  ; Erhu Minigame Initialization and Entry Point
  (`|ExecutionSequence`
    (:`then_0`
      (bind _returnvalue (`|CreateWidget` "/Game/WBP_ErhuHUDLayout.WBP_ErhuHUDLayout_C"))
      (`/Engine/EditorBlueprintResources/StandardMacros.IsValid` _returnvalue
        (:`Is Valid`
          (bind _output_get (set `self.ErhuHUDLayuout` _returnvalue))
          (`UserWidget.AddToViewport` _returnvalue 0)
          (`UserWidget.AddToViewport` _output_get 0)
          (set `PlayerController.bShowMouseCursor` true (`GameplayStatics.GetPlayerController` 0)))))
    (:`then_1`
      (set `self.LeftPerfectHitLocation` (`SceneComponent.K2_GetComponentLocation` (`self.Bullseye`)))
      (set `self.RightPerfectHitLocation` (`SceneComponent.K2_GetComponentLocation` (`self.RightBullseye`))))))

(event `self.NoteDestroyer.OnComponentBeginOverlap`
  (params (OverlappedComponent :type "PrimitiveComponent Object Reference") (OtherActor :type "Actor Object Reference") (OtherComp :type "PrimitiveComponent Object Reference") (OtherBodyIndex :type Integer) (bFromSweep :type Boolean) (SweepResult :type "HitResult Structure (by ref)"))
  ; Lane Note Detection
  ;; Left Lane Hit Detection
  (bind _asbp_music_notes (cast `/Game/BP_MusicNotes` OtherActor))
  (`self.K2_DestroyActor` _asbp_music_notes))

(event `self.BullseyeDetection.OnComponentBeginOverlap`
  (params (OverlappedComponent :type "PrimitiveComponent Object Reference") (OtherActor :type "Actor Object Reference") (OtherComp :type "PrimitiveComponent Object Reference") (OtherBodyIndex :type Integer) (bFromSweep :type Boolean) (SweepResult :type "HitResult Structure (by ref)"))
  ; Lane Note Detection
  ;; Left Lane Hit Detection
  (cast `/Game/BP_MusicNotes` OtherActor)
  (set `self.isNoteOverllapedWithLeftLane` true))

(event `StartCountdown`
  (params (SoundToPlay :type "MetaSoundSource Object Reference"))
  ; Erhu Minigame Initialization and Entry Point
  (set `self.SoundToPl;ay` SoundToPlay)
  (bind _returnvalue (`KismetSystemLibrary.K2_SetTimerDelegate` (delegate `StartMinigame`) (`self.TimeToStart`)))
  (set `self.TimerHandle` _returnvalue)
  (`KismetSystemLibrary.PrintString` "Start Countdown"))

(event `self.BullseyeDetection.OnComponentEndOverlap`
  (params (OverlappedComponent :type "PrimitiveComponent Object Reference") (OtherActor :type "Actor Object Reference") (OtherComp :type "PrimitiveComponent Object Reference") (OtherBodyIndex :type Integer))
  ; Lane Note Detection
  ;; Left Lane Hit Detection
  (bind _asbp_music_notes (cast `/Game/BP_MusicNotes` OtherActor))
  (set `self.isNoteOverllapedWithLeftLane` false))

(event `OnMusicFinish`
  ; Erhu Minigame Initialization and Entry Point
  (`KismetSystemLibrary.K2_ClearAndInvalidateTimerHandle` (`self.TimerHandle`))
  (bind _returnvalue (`GameplayStatics.GetActorOfClass` "/Game/ThirdPerson/Blueprints/BP_ThirdPersonCharacter.BP_ThirdPersonCharacter_C"))
  (`Controller.Possess` (`self.GetController`) _returnvalue)
  (`Widget.RemoveFromParent` (`self.ErhuHUDLayuout`))
  (`self.K2_DestroyActor`)
  (`KismetSystemLibrary.PrintString` "Finish Music"))

(event `StartMinigame`
  (bind _audio (`self.Audio`))
  ; Erhu Minigame Initialization and Entry Point
  (switch `/Game/E_ErhuDifficulty` (`self.DifficultyToPlay`)
    (:`NewEnumerator0`
      (`KismetSystemLibrary.PrintString` "Erhu Minigame start on easy difficulty!"))
    (:`NewEnumerator1`
      (`KismetSystemLibrary.PrintString` "Erhu Minigame start on medium difficulty!"))
    (:`NewEnumerator2`
      (`KismetSystemLibrary.PrintString` "Erhu Minigame start on hard difficulty!")))
  (set `PlayerController.bShowMouseCursor` false (`GameplayStatics.GetPlayerController` 0))
  (`self.EnableInput` (`GameplayStatics.GetPlayerController` 0))
  (`AudioComponent.SetSound` _audio (`self.SoundToPl;ay`))
  (`AudioComponent.Play` _audio 0.0)
  (`MetaSoundOutputSubsystem.WatchOutput` (subsystem `MetaSoundOutputSubsystem`) _audio "Cue Point Label" (delegate `OnSpawningMusicNoteOnCuePoint`) "None" "None")
  (add `AudioComponent.OnAudioFinished` _audio (delegate `OnMusicFinish`)))

(event `self.RightNoteDestroyer.OnComponentBeginOverlap`
  (params (OverlappedComponent :type "PrimitiveComponent Object Reference") (OtherActor :type "Actor Object Reference") (OtherComp :type "PrimitiveComponent Object Reference") (OtherBodyIndex :type Integer) (bFromSweep :type Boolean) (SweepResult :type "HitResult Structure (by ref)"))
  ; Lane Note Detection
  ;; Right Lane Detection
  (bind _asbp_music_notes (cast `/Game/BP_MusicNotes` OtherActor))
  (`self.K2_DestroyActor` _asbp_music_notes))

(event `OnSpawningMusicNoteOnCuePoint`
  (params (OutputName :type Name) (Output :type "MetaSoundOutput Structure (by ref)"))
  ; Erhu Minigame Initialization and Entry Point
  (bind (_success _returnvalue) (`MetasoundOutputBlueprintAccess.GetString` Output))
  (if _success
    (`KismetSystemLibrary.PrintString` "Success Finding Cue Point")
    (switch `string` _returnvalue
      (:`LeftMusicNote`
        (`KismetSystemLibrary.PrintString` _returnvalue)
        (bind _returnvalue_2 (`|SpawnActorFromClass` "/Game/BP_LeftNotes.BP_LeftNotes_C" (`KismetMathLibrary.MakeTransform` (`SceneComponent.K2_GetComponentLocation` (`self.NoteSpawner`))) "Undefined" "MultiplyWithRoot" null null))
        (bind _output_get (set `self.MusicNote` _returnvalue_2))
        (`/Game/BP_MusicNotes.MoveNote` _output_get))
      (:`RightMusicNote`
        (`KismetSystemLibrary.PrintString` _returnvalue)
        (bind _returnvalue_3 (`|SpawnActorFromClass` "/Game/BP_RightNotes.BP_RightNotes_C" (`KismetMathLibrary.MakeTransform` (`SceneComponent.K2_GetComponentLocation` (`self.RightNoteSpawner`))) "Undefined" "MultiplyWithRoot" null null))
        (bind _output_get_2 (set `self.MusicNote` _returnvalue_3))
        (`/Game/BP_MusicNotes.MoveNote` _output_get_2)))))

(event `self.RightBullseyeDetection.OnComponentBeginOverlap`
  (params (OverlappedComponent :type "PrimitiveComponent Object Reference") (OtherActor :type "Actor Object Reference") (OtherComp :type "PrimitiveComponent Object Reference") (OtherBodyIndex :type Integer) (bFromSweep :type Boolean) (SweepResult :type "HitResult Structure (by ref)"))
  ; Lane Note Detection
  ;; Right Lane Detection
  (cast `/Game/BP_MusicNotes` OtherActor)
  (set `self.isNoteOverllapedWithRightLane` true))

(event `self.RightBullseyeDetection.OnComponentEndOverlap`
  (params (OverlappedComponent :type "PrimitiveComponent Object Reference") (OtherActor :type "Actor Object Reference") (OtherComp :type "PrimitiveComponent Object Reference") (OtherBodyIndex :type Integer))
  ; Lane Note Detection
  ;; Right Lane Detection
  (bind _asbp_music_notes (cast `/Game/BP_MusicNotes` OtherActor))
  (set `self.isNoteOverllapedWithRightLane` false))

(event `Key|F`
  (params (Key :type "Key Structure"))
  (bind _bullseye (`self.Bullseye`))
  (bind _rightbullseye (`self.RightBullseye`))
  (:`Pressed`
    (if (`self.isNoteOverllapedWithLeftLane`)
      (set `self.IsInputPressed` true)
      (`PrimitiveComponent.SetMaterial` _bullseye 0 "/DatasmithContent/Materials/AliasReference.AliasReference")
      (`KismetSystemLibrary.Delay` 0.1)
      (`PrimitiveComponent.SetMaterial` _bullseye 0 "/Game/BasicShapeMaterial1.BasicShapeMaterial1")
      (`/Game/ScoreComponent.SetScore` (`self.ScoreComponent`) 1)
      (elif (`self.isNoteOverllapedWithRightLane`)
        (set `self.IsInputPressed` true)
        (`PrimitiveComponent.SetMaterial` _rightbullseye 0 "/DatasmithContent/Materials/AliasReference.AliasReference")
        (`KismetSystemLibrary.Delay` 0.1)
        (`PrimitiveComponent.SetMaterial` _rightbullseye 0 "/Game/BasicShapeMaterial1.BasicShapeMaterial1")
        (`/Game/ScoreComponent.SetScore` (`self.ScoreComponent`) 1)
        (else
          (`KismetSystemLibrary.PrintString` "Missed")))))
  (:`Released`
    (set `self.IsInputPressed` false)))

(fn `GetNoteDistanceToPerfectPoint`
  (params (Distance :type "Float (double-precision)"))
  (returns (IsInputtRIGGERED :type Boolean))
  (if (and (> Distance (`self.NotePerfectWindow`)) (not (`self.IsInputPressed`)))
    (`KismetSystemLibrary.PrintString` "Trigger Game Over")
    (return true)
    (else
      (return false))))

(fn `UserConstructionScript`)