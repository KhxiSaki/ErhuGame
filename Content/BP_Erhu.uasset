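; BP_Erhu is an interactable erhu actor that starts the erhu minigame for a player character entering its box.
; On overlap it prints a prompt and immediately sends the StartErhuMinigame gameplay event to the BP_ThirdPersonCharacter, with itself as instigator.
; A separate Possess event spawns an actor at its transform and hands it to the supplied controller.
; Despite the TriggerSmartObjectBehaviour name, the Smart Object nodes are disconnected and never run.
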(event `self.Box.OnComponentBeginOverlap`
  (params (OverlappedComponent :type "PrimitiveComponent Object Reference") (OtherActor :type "Actor Object Reference") (OtherComp :type "PrimitiveComponent Object Reference") (OtherBodyIndex :type Integer) (bFromSweep :type Boolean) (SweepResult :type "HitResult Structure (by ref)"))
  (`KismetSystemLibrary.PrintString` "You can interact")
  (bind _asbp_third_person_character (cast `/Game/ThirdPerson/Blueprints/BP_ThirdPersonCharacter` OtherActor))
  (`self.TriggerSmartObjectBehaviour` _asbp_third_person_character))

(event `Possess`
  (params (Controller :type "Controller Object Reference"))
  (bind _returnvalue (`|SpawnActorFromClass` "/Game/BP_ErhuActor.BP_ErhuActor_C" (`self.GetTransform`) "Undefined" "MultiplyWithRoot" null null))
  (`/Engine/EditorBlueprintResources/StandardMacros.IsValid` _returnvalue
    (:`Is Valid`
      (`Controller.Possess` Controller _returnvalue))))

(event `TriggerSmartObjectBehaviour`
  (params (Actor :type "Actor Object Reference"))
  (`AbilitySystemBlueprintLibrary.SendGameplayEventToActor` Actor (struct :`TagName` "GameplayEvent.StartErhuMinigame") (make `GameplayEventData` (struct) self Actor)))

(fn `UserConstructionScript`)